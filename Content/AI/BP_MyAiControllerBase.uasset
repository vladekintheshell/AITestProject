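; AI controller base that runs the crocodile combat behavior tree and feeds it target data through the Blackboard.
; Any AI Perception target update, whether sensed or lost, passes the actor to SetEnemy, which stores a changed Enemy and writes it to the Blackboard.
; Each Tick, while controlling a BP_MyMutantBase pawn with an Enemy set, it writes the pawn-to-enemy distance as DistanceToTarget.
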(event OnTargetPerceptionUpdated(AIPerception)
  (params (Actor :type Actor%20Object%20Reference) (Stimulus :type AI%20Stimulus%20Structure))
  ;[1 1 1] Передача New Enemy в функцию Set Enemy
  (CallFunction|SetEnemy Actor))

(event EventBeginPlay
  (AI|RunBehaviorTree "/Game/Blueprints/Characters/Mutants/Crocodile/AI/Behaviors/BT_CrocodileCombatBehavior.BT_CrocodileCombatBehavior"))

(event EventTick
  (params (DeltaSeconds :type Float%20%28single-precision%29))
  ;[1 1 1] Расчет дистанции до цели, который передается в blackboard
  (if (Utilities|IsValid (.AsBP%20My%20Mutant%20Base (Utilities|Casting|CastToBP_MyMutantBase (Pawn|GetControlledPawn self))))
    (if (!= (Variables|Default|GetEnemy) 0)
      (AI|Components|Blackboard|SetValueasFloat (AI|GetBlackboard 0) (Utilities|Name|MakeLiteralName "DistanceToTarget") (Math|Vector|VectorLength (- (Transformation|GetActorLocation (Variables|Default|GetEnemy)) (Transformation|GetActorLocation (Pawn|GetControlledPawn))))))))

(fn ConstructionScript)

(fn SetEnemy
  (params (NewEnemy :type Actor%20Object%20Reference))
  ;[1 1 1] Запись New Enemy в Blackboard
  (if (!= NewEnemy (Variables|Default|GetEnemy))
    (bind _output_get (Variables|Default|SetEnemy NewEnemy))
    (AI|Components|Blackboard|SetValueasObject (AI|GetBlackboard 0) (Utilities|Name|MakeLiteralName "Enemy") _output_get)))