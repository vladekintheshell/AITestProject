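; AI ability for the toxic crocodile's high bite attack.
; Activation plays the high-bite montage, moves the crocodile toward a point straight ahead, and stores the montage length in the blackboard's DelayTime key.
; It then passes the ability's damage to the crocodile's BiteDamage and fires its bite attack call.
; Ending always passes false to the parent and prints a debug string.
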(fn ActivateAvility
  (params (Char :type BP%20My%20Mutant%20Base%20Object%20Reference))
  (bind _returnvalue (AI|GetAIController Char))
  (bind _asbp_toxic_crocodile (Utilities|Casting|CastToBP_ToxicCrocodile Char))
  (bind _asbp_my_ai_controller_base (Utilities|Casting|CastToBP_MyAiControllerBase _returnvalue))
  (|CallParentFunction 0)
  (bind _returnvalue_2 (Animation|PlayAnimMontage Char "/Game/Blueprints/Characters/Mutants/Crocodile/Animations/ANIM_Crocodile_BiteHigh_RM_Montage.ANIM_Crocodile_BiteHigh_RM_Montage" 1.0 "None"))
  (AI|Navigation|SimpleMovetoLocation _asbp_my_ai_controller_base (+ (Transformation|GetActorLocation Char) (* (Transformation|GetActorForwardVector Char) 3.5e+02)))
  (AI|Components|Blackboard|SetValueasFloat (AI|GetBlackboard _asbp_my_ai_controller_base) (Utilities|Name|MakeLiteralName "DelayTime") _returnvalue_2)
  (Default|BiteDamage _asbp_toxic_crocodile 0.0 (Variables|Default|GetDamage))
  (Default|CallBiteAttack _asbp_toxic_crocodile))

(fn OnEndAbility
  (params (Success :type Boolean))
  (|CallParentFunction false)
  (Development|PrintString 0 "EndAbility"))