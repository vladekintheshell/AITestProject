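; Ranged attack ability for the toxic crocodile mutant AI that lobs a projectile at the AI controller's current enemy.
; On activation it solves the ballistic equation from Velocity, Gravity and the horizontal and vertical offsets to the enemy.
; It takes the lower launch angle plus a fixed upward bias as pitch, with yaw from a look-at rotation.
; It passes this transform to BP_ToxicCrocodile's FireProjectile, then immediately ends the ability.
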(fn ActivateAvility
  (params (Char :type BP%20My%20Mutant%20Base%20Object%20Reference))
  (bind _usercharacter (Variables|Default|GetUserCharacter))
  (bind _velocity (Variables|Default|GetVelocity))
  (bind _gravity (Variables|Default|GetGravity))
  (bind _gravity_2 (Variables|Default|GetGravity))
  (bind _usercharacter_2 (Variables|Default|GetUserCharacter))
  (bind _returnvalue (AI|GetAIController _usercharacter))
  (bind _returnvalue_2 (Math|Float|Square _velocity))
  (bind _returnvalue_3 (AI|GetAIController _usercharacter_2))
  (bind _returnvalue_4 (Transformation|GetActorLocation _usercharacter_2))
  (bind _returnvalue_5 (Transformation|GetActorLocation _usercharacter))
  (bind _returnvalue_6 (Math|Float|Square _returnvalue_2))
  (bind _asbp_my_ai_controller_base (Utilities|Casting|CastToBP_MyAiControllerBase _returnvalue_3))
  (bind _asbp_my_ai_controller_base_2 (Utilities|Casting|CastToBP_MyAiControllerBase _returnvalue))
  (bind _enemy (Variables|/Game/AI/BP_MyAiControllerBase.BP_MyAiControllerBase_C|GetEnemy _asbp_my_ai_controller_base_2))
  (bind _enemy_2 (Variables|/Game/AI/BP_MyAiControllerBase.BP_MyAiControllerBase_C|GetEnemy _asbp_my_ai_controller_base))
  (bind _ascharacter (Utilities|Casting|CastToCharacter _enemy_2))
  (bind _ascharacter_2 (Utilities|Casting|CastToCharacter _enemy))
  (bind _returnvalue_7 (Transformation|GetActorLocation _ascharacter))
  (bind _returnvalue_8 (Transformation|GetActorLocation _ascharacter_2))
  (bind _returnvalue_9 (Math|Rotator|FindLookatRotation _returnvalue_5 _returnvalue_8))
  (bind _returnvalue_10 (- (.y _returnvalue_7) (.y _returnvalue_4)))
  (bind _returnvalue_11 (- (.x _returnvalue_7) (.x _returnvalue_4)))
  (bind _returnvalue_12 (- (.z _returnvalue_7) (.z _returnvalue_4)))
  (bind _returnvalue_13 (Math|Vector2D|Vector2DLength (Math|Vector2D|MakeVector2D _returnvalue_10 _returnvalue_11)))
  (bind _returnvalue_14 (* _returnvalue_12 _returnvalue_2))
  (bind _returnvalue_15 (Math|Float|Square _returnvalue_13))
  (bind _returnvalue_16 (* _returnvalue_14 2.0))
  (bind _returnvalue_17 (* _returnvalue_13 _gravity_2))
  (bind _returnvalue_18 (* _returnvalue_15 _gravity_2))
  (bind _returnvalue_19 (+ _returnvalue_18 _returnvalue_16))
  (bind _returnvalue_20 (* _returnvalue_19 _gravity))
  (bind _returnvalue_21 (- _returnvalue_6 _returnvalue_20))
  (bind _returnvalue_22 (Math|Float|Sqrt _returnvalue_21))
  (|CallParentFunction Char)
  ;[1 1 1] Вызов спавна снаряда и передача направления полета.
  (Default|FireProjectile (.AsBP%20Toxic%20Crocodile (Utilities|Casting|CastToBP_ToxicCrocodile _usercharacter)) _returnvalue_5 (Math|Rotator|MakeRotator (.roll _returnvalue_9) (+ (Math|Float|Min(Float) (Class|KismetMathLibrary|DegAtan (/ (+ _returnvalue_22 _returnvalue_2) _returnvalue_17)) (Class|KismetMathLibrary|DegAtan (/ (- _returnvalue_2 _returnvalue_22) _returnvalue_17))) 1e+01) (.yaw _returnvalue_9)))
  (CallFunction|OnEndAbility true))