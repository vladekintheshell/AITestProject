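; Toxic crocodile mutant enemy with a bite attack and a ranged projectile attack, both driven by abilities.
; Bite listens for DamageFace overlaps, damages the first-person player through their damage model, and ends the ability with success or failure after a timer.
; FireProjectile plays a montage and spawns the projectile.
; Damage halts movement during a hit montage, while death unpossesses the crocodile, plays a montage and destroys it.
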(event Custom|BiteAttackOn
  ;[1 1 1] BiteAttackOn вызывается в Bite Ability
  (Collision|AssignOnComponentBeginOverlap (Variables|Default|GetDamageFace) (delegate Custom|OnComponentBeginOverlap_Event_0))
  (Utilities|FlowControl|Delay (Variables|Default|GetAttackTimer))
  ;;[1 1 1] Если Bite не попал по игроку, то Ability завершится с Success False
  (if (not (Variables|Default|GetEnemyGotBite))
    (Default|CallEndAbility false)))

(event Custom|DeathEvent
  (bind _returnvalue (Pawn|GetController))
  ;[1 1 1] Death Event вызывается, когда Health падает <0.
  (Components|DestroyComponent (Variables|Default|GetBP_MyDamageModel))
  (AI|Navigation|StopMovement _returnvalue)
  (Pawn|UnPossess _returnvalue)
  (bind _returnvalue_2 (Animation|PlayAnimMontage "/Game/Blueprints/Characters/Mutants/Crocodile/Animations/ANIM_Crocodile_Death_Montage.ANIM_Crocodile_Death_Montage" 1.0 "None"))
  (Utilities|FlowControl|Delay _returnvalue_2)
  (Actor|DestroyActor)
  (Variables|Default|SetIsDead true))

(event Custom|DamageTaken
  (bind _charactermovement (Variables|Character|GetCharacterMovement))
  ;[1 1 1] Анимация при получении урона.
  (Class|NavMovementComponent|StopActiveMovement _charactermovement)
  (Pawn|Components|CharacterMovement|DisableMovement _charactermovement)
  (bind _returnvalue (Animation|PlayAnimMontage "/Game/Blueprints/Characters/Mutants/Crocodile/Animations/ANIM_Crocodile_GetHit_Montage.ANIM_Crocodile_GetHit_Montage" 1.0 "None"))
  (Utilities|FlowControl|Delay _returnvalue)
  (Pawn|Components|CharacterMovement|SetMovementMode _charactermovement "MOVE_Walking" 0))

(event Custom|OnComponentBeginOverlap_Event_0
  (params (OverlappedComponent :type Primitive%20Component%20Object%20Reference) (OtherActor :type Actor%20Object%20Reference) (OtherComp :type Primitive%20Component%20Object%20Reference) (OtherBodyIndex :type Integer) (bFromSweep :type Boolean) (SweepResult :type Hit%20Result%20Structure%20%28by%20ref%29))
  (bind _asfirst_person_character (Utilities|Casting|CastToFirstPersonCharacter OtherActor))
  ;[1 1 1] BiteAttackOn вызывается в Bite Ability
  ;;[1 1 1] Если Bite попал по игроку, то ему нанесется урон, а Ability завершится с Success True.
  (if (== OtherActor _asfirst_person_character)
    (Variables|Default|SetEnemyGotBite true)
    (Utilities|FlowControl|DoOnce false :!label _label
      (:Completed
        (Default|DamageReceived (Variables|/Game/FirstPersonBP/Blueprints/FirstPersonCharacter.FirstPersonCharacter_C|GetBP_MyDamageModel _asfirst_person_character) (Variables|Default|GetBiteDamageAmount))
        (Utilities|FlowControl|Delay (Variables|Default|GetAttackTimer))
        (EventDispatchers|UnbindallEventsfromOnComponentBeginOverlap (Variables|Default|GetDamageFace))
        (Default|CallEndAbility true)
        (Variables|Default|SetEnemyGotBite false)
        (goto _label Reset)))))

(event EventBeginPlay
  (|CallParentFunction)
  (Utilities|FlowControl|Sequence
    (:then_0
      ;[1 1 1] Death Event вызывается, когда Health падает <0.
      (EventDispatchers|AssignDeathEvent (Variables|Default|GetBP_MyDamageModel) (delegate Custom|DeathEvent)))
    (:then_1
      ;[1 1 1] BiteAttackOn вызывается в Bite Ability
      (EventDispatchers|BindEventtoBiteAttack (delegate Custom|BiteAttackOn)))
    (:then_2
      ;[1 1 1] Анимация при получении урона.
      (EventDispatchers|BindEventtoGotDamage (delegate Custom|DamageTaken)))))

(event Collision|EventActorBeginOverlap
  (params (OtherActor :type Actor%20Object%20Reference))
  (|CallParentFunction OtherActor) ; This node is disabled and will not be called.\nDrag off pins to build functionality.
)

(fn ConstructionScript
  (|CallParentFunction))

(fn FireProjectile
  (params (SpawnTransformLocation :type Vector) (SpawnTransormRotation :type Rotator))
  ;[1 1 1] Вызов спавна снаряда для Range Ability.
  (Animation|PlayAnimMontage "/Game/Blueprints/Characters/Mutants/Crocodile/Animations/ANIM_Crocodile_BiteHigh_RM_Montage.ANIM_Crocodile_BiteHigh_RM_Montage" 1.0 "None")
  (Game|SpawnActorfromClass "/Game/Blueprints/Characters/Mutants/Crocodile/Projectile/BP_RangeAttackProjectile.BP_RangeAttackProjectile_C" (Math|Transform|MakeTransform SpawnTransformLocation SpawnTransormRotation "0.300000,0.300000,0.300000") "Undefined" 0 0))

(fn BiteDamage
  (params (AttackTimer :type Float%20%28single-precision%29) (BiteDamage :type Float%20%28single-precision%29))
  (Variables|Default|SetAttackTimer AttackTimer)
  (Variables|Default|SetBiteDamageAmount BiteDamage))