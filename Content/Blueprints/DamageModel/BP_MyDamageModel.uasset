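; BP_MyDamageModel is a health model that handles damage, healing and death notification.
; On BeginPlay it stores the starting Health as MaxHealth.
; DamageReceived subtracts damage without clamping and calls the death event whenever Health is zero or below.
; Heal adds health capped at MaxHealth and only works while Health is non-negative, so exactly zero can still be healed.
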(event EventBeginPlay
  ;[1 1 1] На старте игры Max Health == Health. Сделано для того, чтобы не плодить лишних переменных.
  (Variables|Default|SetMaxHealth (Variables|Default|GetHealth)))

(event EventTick
  (params (DeltaSeconds :type Float%20%28single-precision%29)))

(fn Heal
  (params (Heal :type Float%20%28single-precision%29))
  ;[1 1 1] Функция, которая при вызове добавляет к Health количество восстановленного здоровья из Heal. В случае, если после Heal количество Health привысит Max Health, Health будет приведено к Max Health.
  (if (>= (Variables|Default|GetHealth) 0.0)
    (Variables|Default|SetHealth (+ (Variables|Default|GetHealth) Heal))
    (if (> (Variables|Default|GetHealth) (Variables|Default|GetMaxHealth))
      (Variables|Default|SetHealth (Variables|Default|GetMaxHealth)))))

(fn DamageReceived
  (params (DamageAmount :type Float%20%28single-precision%29))
  ;[1 1 1] Функция, которая при вызове отнимает от Health количество полученного урона. В случае, если Health упадет ниже 0 после получения урона, будет вызван Death Event.
  (Variables|Default|SetHealth (- (Variables|Default|GetHealth) DamageAmount))
  (if (<= (Variables|Default|GetHealth) 0.0)
    (Default|CallDeathEvent)))