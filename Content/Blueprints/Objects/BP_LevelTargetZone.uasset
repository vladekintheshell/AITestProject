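; BP_LevelTargetZone is a level objective actor that ends the game once the required number of crocodile kills is reached.
; On BeginPlay it binds one handler to the death events of two referenced crocodiles through their damage model components.
; Each death decrements the NeedToKill counter, and at zero it calls CallEndGame on the FirstPersonCharacter.
; Despite the zone name, it has no active overlap logic.
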(event Custom|Dead1
  (Math|Integer|DecrementInt (Variables|Default|GetNeedToKill)
    (:%20%20
      (if (== (Variables|Default|GetNeedToKill) 0)
        (Default|CallEndGame (.AsFirst%20Person%20Character (Utilities|Casting|CastToFirstPersonCharacter (Game|GetPlayerCharacter 0))))))))

(event EventBeginPlay
  (EventDispatchers|AssignDeathEvent (Variables|/Game/Characters/Mutants/BP_MyMutantBase.BP_MyMutantBase_C|GetBP_MyDamageModel (Variables|Default|GetCrocodile1)) (delegate Custom|Dead1))
  (EventDispatchers|AssignDeathEvent (Variables|/Game/Characters/Mutants/BP_MyMutantBase.BP_MyMutantBase_C|GetBP_MyDamageModel (Variables|Default|GetCrocodile2)) (delegate Custom|Dead1)))

(event Collision|EventActorBeginOverlap
  (params (OtherActor :type Actor%20Object%20Reference)))

(event EventTick
  (params (DeltaSeconds :type Float%20%28single-precision%29)))

(fn ConstructionScript)