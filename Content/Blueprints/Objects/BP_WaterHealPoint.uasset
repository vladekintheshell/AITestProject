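; BP_WaterHealPoint is a healing zone that periodically restores health to a BP_ToxicCrocodile inside its Box.
; Box overlap events store the crocodile reference on entry and clear it on exit.
; While that reference is valid, Tick runs a Delay that throttles Heal calls on the crocodile's BPMyDamageModel to roughly once per second.
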(event OnComponentBeginOverlap(Box)
  (params (OverlappedComponent :type Primitive%20Component%20Object%20Reference) (OtherActor :type Actor%20Object%20Reference) (OtherComp :type Primitive%20Component%20Object%20Reference) (OtherBodyIndex :type Integer) (bFromSweep :type Boolean) (SweepResult :type Hit%20Result%20Structure%20%28by%20ref%29))
  (bind _asbp_toxic_crocodile (Utilities|Casting|CastToBP_ToxicCrocodile OtherActor))
  (if (== OtherActor _asbp_toxic_crocodile)
    (Variables|Default|SetAs%20BP%20Toxic%20Crocodile _asbp_toxic_crocodile)))

(event OnComponentEndOverlap(Box)
  (params (OverlappedComponent :type Primitive%20Component%20Object%20Reference) (OtherActor :type Actor%20Object%20Reference) (OtherComp :type Primitive%20Component%20Object%20Reference) (OtherBodyIndex :type Integer))
  (if (== OtherActor (.AsBP%20Toxic%20Crocodile (Utilities|Casting|CastToBP_ToxicCrocodile OtherActor)))
    (Variables|Default|SetAs%20BP%20Toxic%20Crocodile 0)))

(event EventBeginPlay)

(event Collision|EventActorBeginOverlap
  (params (OtherActor :type Actor%20Object%20Reference)))

(event EventTick
  (params (DeltaSeconds :type Float%20%28single-precision%29))
  (bind _as_bp_toxic_crocodile (Variables|Default|GetAs%20BP%20Toxic%20Crocodile))
  ;[1 1 1] Переодическое лечение персонажа Крокодила, пока он находится в области WaterHealPoint.
  (if (Utilities|IsValid _as_bp_toxic_crocodile)
    (Utilities|FlowControl|Delay 1.0)
    (Default|Heal (Variables|/Game/Characters/Mutants/BP_MyMutantBase.BP_MyMutantBase_C|GetBP_MyDamageModel _as_bp_toxic_crocodile) 25.0)))

(fn ConstructionScript)